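; A pushable VR button that latches or toggles, with callable push, pull, toggle and reset events.
; Hits above an impulse threshold along its up axis, or optional overlaps, trigger it through a DoOnce gate reset by a cooldown timeline.
; Push and pull timelines slide the mesh and blend a dynamic material between pushed and pulled colors, with a sound played on push.
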(event Custom|OnComponentBeginOverlap_Event_0
  (params (OtherActor :type Actor%20Object%20Reference) (OtherComp :type Primitive%20Component%20Object%20Reference) (OtherBodyIndex :type Integer) (bFromSweep :type Boolean) (SweepResult :type Hit%20Result%20Structure%20%28by%20ref%29))
  (bind _colorpushed (Variables|Default|GetColorPushed))
  (bind _colorpulled (Variables|Default|GetColorPulled))
  (bind _button_material (Variables|Default|GetButton%20Material))
  (bind _button_mesh (Variables|Default|GetButton%20Mesh))
  (bind _pressdepth (Variables|Default|GetPressDepth))
  (if (Variables|Default|GetEnableOverlapPush)
    (Utilities|FlowControl|DoOnce false :!label _label
      (:Completed
        (Utilities|FlowControl|Sequence
          (:then_0
            (Timeline|cooldown PlayFromStart
              (:Finished
                (goto _label Reset))))
          (:then_1
            (if (Variables|Default|GetToggleOrPush)
              (if (not (Variables|Default|GetButton%20Pushed))
                (Variables|Default|SetButton%20Pushed true :!label _label_2)
                (Utilities|FlowControl|Sequence
                  (:then_0
                    (Utilities|FlowControl|DoOnce false :!label _label_3
                      (:Completed
                        (Audio|PlaySoundatLocation (Variables|Default|GetButtonSound) (Transformation|GetWorldLocation _button_mesh)))))
                  (:then_1
                    (bind _newtrack_0 (Timeline|PushAnim PlayFromStart)
                      (:Update
                        (Transformation|SetRelativeLocation _button_mesh (Math|Vector|MakeVector 0.0 0.0 (* (- _newtrack_0 1.0) _pressdepth 1e+01)) false true)
                        (Rendering|Material|SetVectorParameterValue _button_material "Color" (Math|Color|Lerp(LinearColor) _colorpushed _colorpulled _newtrack_0) :!class /Script/Engine.MaterialInstanceDynamic))))))
              (elif (Variables|Default|GetButton%20Pushed)
                (Variables|Default|SetButton%20Pushed false)
                (Utilities|FlowControl|Sequence
                  (:then_0
                    (goto _label_3 Reset))
                  (:then_2
                    (bind _newtrack_0_2 (Timeline|PullAnim PlayFromStart)
                      (:Update
                        (Transformation|SetRelativeLocation _button_mesh (Math|Vector|MakeVector 0.0 0.0 (* (- _newtrack_0_2 1.0) _pressdepth 1e+01)) false true)
                        (Rendering|Material|SetVectorParameterValue _button_material "Color" (Math|Color|Lerp(LinearColor) _colorpushed _colorpulled _newtrack_0_2) :!class /Script/Engine.MaterialInstanceDynamic)))))
                (else
                  (goto _label_2))))))))))

(event Custom|ButtonPush
  (bind _button_mesh (Variables|Default|GetButton%20Mesh))
  (if (not (Variables|Default|GetButton%20Pushed))
    (Variables|Default|SetButton%20Pushed true)
    (Utilities|FlowControl|Sequence
      (:then_0
        (Utilities|FlowControl|DoOnce false
          (:Completed
            (Audio|PlaySoundatLocation (Variables|Default|GetButtonSound) (Transformation|GetWorldLocation _button_mesh)))))
      (:then_1
        (bind _newtrack_0 (Timeline|PushAnim PlayFromStart)
          (:Update
            (Transformation|SetRelativeLocation _button_mesh (Math|Vector|MakeVector 0.0 0.0 (* (- _newtrack_0 1.0) (Variables|Default|GetPressDepth) 1e+01)) false true)
            (Rendering|Material|SetVectorParameterValue (Variables|Default|GetButton%20Material) "Color" (Math|Color|Lerp(LinearColor) (Variables|Default|GetColorPushed) (Variables|Default|GetColorPulled) _newtrack_0) :!class /Script/Engine.MaterialInstanceDynamic)))))))

(event Custom|ButtonPull
  (bind _button_mesh (Variables|Default|GetButton%20Mesh))
  (if (Variables|Default|GetButton%20Pushed)
    (Variables|Default|SetButton%20Pushed false)
    (Utilities|FlowControl|Sequence
      (:then_0
        (Utilities|FlowControl|DoOnce false) ; enters at Reset
      )
      (:then_2
        (bind _newtrack_0 (Timeline|PullAnim PlayFromStart)
          (:Update
            (Transformation|SetRelativeLocation _button_mesh (Math|Vector|MakeVector 0.0 0.0 (* (- _newtrack_0 1.0) (Variables|Default|GetPressDepth) 1e+01)) false true)
            (Rendering|Material|SetVectorParameterValue (Variables|Default|GetButton%20Material) "Color" (Math|Color|Lerp(LinearColor) (Variables|Default|GetColorPushed) (Variables|Default|GetColorPulled) _newtrack_0) :!class /Script/Engine.MaterialInstanceDynamic)))))))

(event Custom|OnComponentHit_Event_1
  (params (OtherActor :type Actor%20Object%20Reference) (OtherComp :type Primitive%20Component%20Object%20Reference) (NormalImpulse :type Vector) (Hit :type Hit%20Result%20Structure%20%28by%20ref%29))
  (bind _colorpushed (Variables|Default|GetColorPushed))
  (bind _colorpulled (Variables|Default|GetColorPulled))
  (bind _button_material (Variables|Default|GetButton%20Material))
  (bind _button_mesh (Variables|Default|GetButton%20Mesh))
  (bind _pressdepth (Variables|Default|GetPressDepth))
  (if (Variables|Default|GetEnableCollisionPush)
    (if (> (Math|Float|Absolute(Float) (Math|Vector|DotProduct NormalImpulse (Math|Vector|GetUpVector (Variables|Default|GetDefaultSceneRoot)))) (Variables|Default|GetCollisionPushThreshold))
      (Utilities|FlowControl|DoOnce false :!label _label
        (:Completed
          (Utilities|FlowControl|Sequence
            (:then_0
              (Timeline|cooldown PlayFromStart
                (:Finished
                  (goto _label Reset))))
            (:then_1
              (if (Variables|Default|GetToggleOrPush)
                (if (not (Variables|Default|GetButton%20Pushed))
                  (Variables|Default|SetButton%20Pushed true :!label _label_2)
                  (Utilities|FlowControl|Sequence
                    (:then_0
                      (Utilities|FlowControl|DoOnce false :!label _label_3
                        (:Completed
                          (Audio|PlaySoundatLocation (Variables|Default|GetButtonSound) (Transformation|GetWorldLocation _button_mesh)))))
                    (:then_1
                      (bind _newtrack_0 (Timeline|PushAnim PlayFromStart)
                        (:Update
                          (Transformation|SetRelativeLocation _button_mesh (Math|Vector|MakeVector 0.0 0.0 (* (- _newtrack_0 1.0) _pressdepth 1e+01)) false true)
                          (Rendering|Material|SetVectorParameterValue _button_material "Color" (Math|Color|Lerp(LinearColor) _colorpushed _colorpulled _newtrack_0) :!class /Script/Engine.MaterialInstanceDynamic))))))
                (elif (Variables|Default|GetButton%20Pushed)
                  (Variables|Default|SetButton%20Pushed false)
                  (Utilities|FlowControl|Sequence
                    (:then_0
                      (goto _label_3 Reset))
                    (:then_2
                      (bind _newtrack_0_2 (Timeline|PullAnim PlayFromStart)
                        (:Update
                          (Transformation|SetRelativeLocation _button_mesh (Math|Vector|MakeVector 0.0 0.0 (* (- _newtrack_0_2 1.0) _pressdepth 1e+01)) false true)
                          (Rendering|Material|SetVectorParameterValue _button_material "Color" (Math|Color|Lerp(LinearColor) _colorpushed _colorpulled _newtrack_0_2) :!class /Script/Engine.MaterialInstanceDynamic)))))
                  (else
                    (goto _label_2)))))))))))

(event Custom|ButtonToggle
  (bind _colorpushed (Variables|Default|GetColorPushed))
  (bind _colorpulled (Variables|Default|GetColorPulled))
  (bind _button_material (Variables|Default|GetButton%20Material))
  (bind _button_mesh (Variables|Default|GetButton%20Mesh))
  (bind _pressdepth (Variables|Default|GetPressDepth))
  (if (Variables|Default|GetButton%20Pushed)
    (Variables|Default|SetButton%20Pushed false)
    (Utilities|FlowControl|Sequence
      (:then_0
        (goto _label Reset))
      (:then_2
        (bind _newtrack_0 (Timeline|PullAnim PlayFromStart)
          (:Update
            (Transformation|SetRelativeLocation _button_mesh (Math|Vector|MakeVector 0.0 0.0 (* (- _newtrack_0 1.0) _pressdepth 1e+01)) false true)
            (Rendering|Material|SetVectorParameterValue _button_material "Color" (Math|Color|Lerp(LinearColor) _colorpushed _colorpulled _newtrack_0) :!class /Script/Engine.MaterialInstanceDynamic)))))
    (else
      (Variables|Default|SetButton%20Pushed true)
      (Utilities|FlowControl|Sequence
        (:then_0
          (Utilities|FlowControl|DoOnce false :!label _label
            (:Completed
              (Audio|PlaySoundatLocation (Variables|Default|GetButtonSound) (Transformation|GetWorldLocation _button_mesh)))))
        (:then_1
          (bind _newtrack_0_2 (Timeline|PushAnim PlayFromStart)
            (:Update
              (Transformation|SetRelativeLocation _button_mesh (Math|Vector|MakeVector 0.0 0.0 (* (- _newtrack_0_2 1.0) _pressdepth 1e+01)) false true)
              (Rendering|Material|SetVectorParameterValue _button_material "Color" (Math|Color|Lerp(LinearColor) _colorpushed _colorpulled _newtrack_0_2) :!class /Script/Engine.MaterialInstanceDynamic))))))))

(event Custom|ButtonReset
  (bind _button_mesh (Variables|Default|GetButton%20Mesh))
  (Variables|Default|SetButton%20Pushed false)
  (Utilities|FlowControl|Sequence
    (:then_0
      (Utilities|FlowControl|DoOnce false) ; enters at Reset
    )
    (:then_2
      (bind _newtrack_0 (Timeline|PullAnim PlayFromStart)
        (:Update
          (Transformation|SetRelativeLocation _button_mesh (Math|Vector|MakeVector 0.0 0.0 (* (- _newtrack_0 1.0) (Variables|Default|GetPressDepth) 1e+01)) false true)
          (Rendering|Material|SetVectorParameterValue (Variables|Default|GetButton%20Material) "Color" (Math|Color|Lerp(LinearColor) (Variables|Default|GetColorPushed) (Variables|Default|GetColorPulled) _newtrack_0) :!class /Script/Engine.MaterialInstanceDynamic))))))

(event EventTick
  (params (DeltaSeconds :type Float%20%28single-precision%29)))

(event EventBeginPlay
  (bind _button_material (Variables|Default|GetButton%20Material))
  (bind _button_mesh (Variables|Default|GetButton%20Mesh))
  (Collision|AssignOnComponentBeginOverlap _button_mesh (delegate Custom|OnComponentBeginOverlap_Event_0))
  (Collision|AssignOnComponentHit _button_mesh (delegate Custom|OnComponentHit_Event_1))
  (if (Variables|Default|GetButton%20Pushed)
    (Rendering|Material|SetVectorParameterValue _button_material "Color" (Variables|Default|GetColorPushed) :!class /Script/Engine.MaterialInstanceDynamic)
    (else
      (Rendering|Material|SetVectorParameterValue _button_material "Color" (Variables|Default|GetColorPulled) :!class /Script/Engine.MaterialInstanceDynamic))))

(fn ConstructionScript
  (bind _returnvalue (Rendering|Material|CreateDynamicMaterialInstance (Variables|Default|GetButton%20Mesh) 0 "/Game/VRDemo_Assets/Materials/BP_Button_INST.BP_Button_INST" :!class /Script/Engine.PrimitiveComponent))
  (Variables|Default|SetButton%20Material _returnvalue))