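; VR demo board actor that displays the player's subscribed Steam Workshop mods, fetched on BeginPlay.
; UpdateModList joins uppercased names, passed through CutString, into one text block capped at MaxLines with an ellipsis, then scales it uniformly to fit the board mesh.
; With no mods, it either hides the board or shows the NoMods message, depending on HideOnZeroMods.
; The construction script sets board width.
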(event Custom|UpdateModList
  (bind _modlist (Variables|Default|GetModList))
  (bind _staticmesh (Variables|Default|GetStaticMesh))
  (bind _listtest (Variables|Default|GetListTest))
  (bind _returnvalue (Utilities|Array|Length _modlist))
  (bind _returnvalue_2 (Class|TextRenderComponent|GetTextLocalSize _listtest))
  (bind _returnvalue_3 (Transformation|GetWorldScale _staticmesh))
  (bind (_x _y _z) (Math|Vector|BreakVector _returnvalue_2))
  (bind _returnvalue_4 (== _returnvalue 0))
  (bind (_x_2 _y_2) (Math|Vector|BreakVector _returnvalue_3))
  (Utilities|FlowControl|Sequence
    (:then_0
      ;[1 1 1] no mods message or hide board
      (if (Variables|Default|GetHideOnZeroMods)
        (Rendering|SetVisibility (Variables|Default|GetNoMods) false false)
        (if _returnvalue_4
          (Rendering|SetActorHiddenInGame true)
          (Collision|SetActorEnableCollision false)
          (else
            (Rendering|SetActorHiddenInGame false)
            (Collision|SetActorEnableCollision true)))
        (else
          (Rendering|SetActorHiddenInGame false)
          (if _returnvalue_4
            (Rendering|SetVisibility (Variables|Default|GetNoMods) true false)
            (else
              (Rendering|SetVisibility (Variables|Default|GetNoMods) false false))))))
    (:then_1
      ;[1 1 1] make a list string
      (Variables|Default|Setdisplaylist "")
      (bind (_array_element _array_index) (Utilities|Array|ForEachLoopwithBreak (Variables|Default|GetModList) :!label _label)
        (:LoopBody
          (Math|Integer|CompareInt _array_index (Variables|Default|GetMaxLines)
            (:>
              (goto _label Break))
            (:==
              (Variables|Default|Setdisplaylist (Utilities|String|Append (Variables|Default|Getdisplaylist) "...")))
            (:<
              (Variables|Default|Setdisplaylist (Utilities|String|Append (Variables|Default|Getdisplaylist) (Utilities|String|Append (Utilities|CutString (Class|KismetStringLibrary|ToUpper _array_element) (Variables|Default|GetMaxStringLength)) " 
"))))))
        (:Completed
          ;[1 1 1] scale to fit the board
          (Rendering|Components|TextRender|SetText _listtest (Utilities|Text|ToText(String) (Variables|Default|Getdisplaylist)))
          (Transformation|SetWorldScale3D _listtest (* "1.000000,1.000000,1.000000" (Math|Float|Min(Float) (/ (* _x_2 3e+02) _y) (/ (* _y_2 1.8e+02) _z)))))))))

(event EventBeginPlay
  (Variables|Default|SetModList (CallFunction|GetSteamWorkshopSubscribedItems))
  (CallFunction|UpdateModList))

(event EventActorBeginOverlap
  (params (OtherActor :type Actor%20Object%20Reference)))

(event EventTick
  (params (DeltaSeconds :type Float%20%28single-precision%29)))

(fn ConstructionScript
  (Transformation|SetRelativeScale3D (Variables|Default|GetStaticMesh) (Math|Vector|MakeVector (Variables|Default|GetWidth) 1.0 1.0)))