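; Blueprint Interface for VR motion controllers in the VR demo, declaring the messages exchanged with controller Blueprints.
; Input functions pass trigger, grip, thumbstick, face and shoulder button states.
; Setup functions pass controller tag, handedness, gun damage and emitters, plus VR options such as crosshair, teleportation and stick locomotion.
; A hit reporter takes a hit actor and location and returns a location vector.
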(fn TriggerBoolean
  (params (Triggered :type Boolean))
  (return false))

(fn TriggerFloat
  (params (Trigger%20Axis :type Float%20%28single-precision%29))
  (return false))

(fn ControllerTag
  (params (Controller%20Tag :type Name))
  (return false))

(fn ControllerSettings
  (params (Muzzle%20Emitter :type Particle%20System%20Object%20Reference) (Flex%20Emitter%20 :type Particle%20System%20Object%20Reference) (Is%20Right? :type Boolean) (Use%20Gamepad? :type Boolean) (Gun%20Base%20Damage :type Float%20%28single-precision%29) (Gun%20Damage%20Radius :type Float%20%28single-precision%29) (Gun%20Impulse%20Strength :type Float%20%28single-precision%29))
  (return false))

(fn HitActorReporter
  (params (Report%20Hit%20Actor :type Actor%20Object%20Reference) (Report%20Hit%20Actor%20Location :type Vector))
  (return 0 ""))

(fn GetVRSettings
  (params (Change%20Settings :type Boolean) (Use%20This%20Controller%20Interface? :type Boolean) (Use%20HUD%20Crosshair%20In%20Dev%20Mode? :type Boolean) (Hud%20Crosshair%20Texture :type Texture%20Object%20Reference) (Location%20Offset :type Vector) (Controller%20Scale%20Value :type Vector) (Controller%20Blueprints%20L-R :type Array%20of%20Actor%20Class%20References) (Gun%20Muzzle%20Emitter :type Particle%20System%20Object%20Reference) (Gun%20Base%20Damage :type Float%20%28single-precision%29) (Gun%20Damage%20Radius :type Float%20%28single-precision%29) (Gun%20Impulse%20Strength :type Float%20%28single-precision%29) (Flex%20Particle%20System :type Particle%20System%20Object%20Reference) (Use%20Trigger%20L%20Axis :type Boolean) (Use%20Trigger%20R%20Axis :type Boolean) (SpawnOwner :type Actor%20Object%20Reference) (Disable%20Low%20Latency%20Update :type Boolean) (Allow%20Teleportation? :type Boolean) (Use%20Stick%20Locomotion? :type Boolean))
  (return false))

(fn FaceButtonBooleans
  (params (Pressed? :type Boolean))
  (return false))

(fn GripBoolean
  (params (Gripped :type Boolean))
  (return false))

(fn ThumbstickBooleans
  (return false))

(fn GripFloats
  (params (Grip%20Float :type Float%20%28single-precision%29))
  (return false))

(fn ThumbstickFloats
  (return false))

(fn ShoulderButtonBooleans
  (params (Pushed :type Boolean) (Is%20Right? :type Boolean))
  (return false))