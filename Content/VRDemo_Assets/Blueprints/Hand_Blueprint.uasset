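; VR hand actor that animates a skeletal hand as either left or right, chosen by IsRight.
; On first tick it copies the left-hand transform if needed, enables input and freezes a single pose animation.
; PlayFromTo scrubs that animation between pose positions with an eased Timeline.
; Matching trigger and face button drive empty grab and pointing, while UpdatePose handles idle, grab and grip, scaling grab and grip by Factor.
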(event Custom|BeginTick
  (bind _skeletalhandl (Variables|Default|GetSkeletalHandL))
  (bind _skeletalhandr (Variables|Default|GetSkeletalHandR))
  (bind _isright (Variables|Default|GetIsRight))
  (bind _skeletalhandr_2 (Variables|Default|GetSkeletalHandR))
  (bind _returnvalue (Transformation|GetRelativeTransform _skeletalhandl))
  (Utilities|FlowControl|Sequence
    (:then_0
      (Transformation|SetRelativeTransform (Variables|Default|GetHandR_Collider) (Math|Transform|SelectTransform (Transformation|GetRelativeTransform _skeletalhandr) _returnvalue _isright) false true)
      ;[1 1 1] switch to left hand
      (if (not _isright)
        (Transformation|SetRelativeTransform _skeletalhandr _returnvalue false true)))
    (:then_1
      (Input|EnableInput (Game|GetPlayerController 0)))
    (:then_2
      ;[1 1 1] start animation and stop immediately (required to be able to set position from bp?)
      (Components|Animation|PlayAnimation _skeletalhandr_2 "/Game/VRDemo_Assets/Meshes/hand_animation2_Anim.hand_animation2_Anim" false)
      (Components|Timeline|SetPlayRate _skeletalhandr_2 0.0)
      ;[1 1 1] wtf exported mesh offset compensation?
      (Transformation|AddLocalOffset _skeletalhandr_2 "4.000000, 0, 0" false false))))

(event Custom|UpdatePose
  (params (Pose :type String) (Factor :type Float%20%28single-precision%29))
  ;[1 1 1] switching poses
  (Variables|Default|SetPreviousPose (Variables|Default|GetCurrentPose))
  (bind _output_get (Variables|Default|SetCurrentPose Pose))
  (switch string _output_get
    (:idle
      (switch string (Variables|Default|GetPreviousPose)
        (:grab
          _)
        (:grip
          _))
      (CallFunction|Playfromto (Class|SkeletalMeshComponent|GetPosition (Variables|Default|GetSkeletalHandR)) 6.0))
    (:highlight
      (switch string (Variables|Default|GetPreviousPose)))
    (:grab
      (CallFunction|Playfromto 2.0 (Math|Float|MapRangeClamped Factor 5.0 3e+01 5.0 2.0)))
    (:grip
      (CallFunction|Playfromto 6.0 (Math|Float|MapRangeClamped Factor 0.0 1.0 9.0 7.0)))))

(event Custom|PlayFromTo
  (params (From :type Float%20%28single-precision%29) (To :type Float%20%28single-precision%29))
  ;[1 1 1] interpolate function
  (Variables|Default|SetIsPlaying true)
  (bind _newtrack_0 (Timeline|Timeline_0 PlayFromStart)
    (:Update
      (Components|Animation|SetPosition (Variables|Default|GetSkeletalHandR) (/ (Math|Float|Lerp From To (|(((3-(2*A))*A)*A) _newtrack_0)) 2.398) false))
    (:Finished
      (Variables|Default|SetIsPlaying false))))

(event EventBeginPlay)

(event EventActorBeginOverlap
  (params (OtherActor :type Actor%20Object%20Reference)))

(event EventTick
  (params (DeltaSeconds :type Float%20%28single-precision%29))
  (Utilities|FlowControl|Sequence
    (:then_0
      (Utilities|FlowControl|DoOnce false
        (:Completed
          (CallFunction|BeginTick))))))

(event Input|KeyboardEvents|MotionControllerLeftFaceButton1
  (params (Key :type Key%20Structure))
  (bind _fingerpointing (Variables|Default|GetFingerPointing))
  ;[1 1 1] empty pointer
  (:Pressed
    (if _fingerpointing
      (if (not (Variables|Default|GetIsRight))
        (CallFunction|Playfromto 1e+01 11.0))))
  (:Released
    (if _fingerpointing
      (if (not (Variables|Default|GetIsRight))
        (CallFunction|Playfromto 11.0 1e+01)))))

(event Input|KeyboardEvents|MotionControllerRightFaceButton1
  (params (Key :type Key%20Structure))
  (bind _fingerpointing (Variables|Default|GetFingerPointing))
  ;[1 1 1] empty pointer
  (:Pressed
    (if _fingerpointing
      (if (Variables|Default|GetIsRight)
        (CallFunction|Playfromto 1e+01 11.0))))
  (:Released
    (if _fingerpointing
      (if (Variables|Default|GetIsRight)
        (CallFunction|Playfromto 11.0 1e+01)))))

(event Input|KeyboardEvents|MotionControllerLeftTrigger
  (params (Key :type Key%20Structure))
  ;[1 1 1] empty grab
  (:Pressed
    (if (not (Variables|Default|GetIsRight))
      (CallFunction|Playfromto 1e+01 9.0)))
  (:Released
    (if (not (Variables|Default|GetIsRight))
      (CallFunction|Playfromto 9.0 1e+01))))

(event Input|KeyboardEvents|MotionControllerRightTrigger
  (params (Key :type Key%20Structure))
  ;[1 1 1] empty grab
  (:Pressed
    (if (Variables|Default|GetIsRight)
      (CallFunction|Playfromto 1e+01 9.0)))
  (:Released
    (if (Variables|Default|GetIsRight)
      (CallFunction|Playfromto 9.0 1e+01))))

(fn ConstructionScript)