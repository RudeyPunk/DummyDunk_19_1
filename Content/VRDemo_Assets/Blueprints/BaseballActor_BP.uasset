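; Baseball actor in the VR demo that plays impact sounds scaled to how hard it hits.
; Hit events feed a frameTest gate checked on Tick, which triggers both cues at the hit location when ready.
; Impulse magnitude sets each volume, layering the hard cue over the soft one only on stronger impacts.
; An older threshold-and-DoOnce version remains in the graph, disconnected.
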(event Collision|EventHit
  (params (MyComp :type Primitive%20Component%20Object%20Reference) (Other :type Actor%20Object%20Reference) (OtherComp :type Primitive%20Component%20Object%20Reference) (bSelfMoved :type Boolean) (HitLocation :type Vector) (HitNormal :type Vector :default "0, 0, 0") (NormalImpulse :type Vector) (Hit :type Hit%20Result%20Structure%20%28by%20ref%29))
  (bind _returnvalue (Math|Vector|VectorLength NormalImpulse))
  ;[1 1 1] Blend Audio Cues
  (Utilities|FrameTest 2) ; enters at Hit
)

(event EventBeginPlay)

(event EventActorBeginOverlap
  (params (OtherActor :type Actor%20Object%20Reference)))

(event EventTick
  (params (DeltaSeconds :type Float%20%28single-precision%29))
  ;[1 1 1] Blend Audio Cues
  (Utilities|FrameTest 2
    (:Ready
      (Utilities|FlowControl|Sequence
        (:then_0
          (Audio|PlaySoundatLocation "/Game/VRDemo_Assets/Audio/baseballimpact_hard_Cue.baseballimpact_hard_Cue" (stale Collision|EventHit HitLocation) "0, 0, 0" (Math|Float|Clamp(Float) (/ (- (Math|Vector|VectorLength (stale Collision|EventHit NormalImpulse)) 2e+03) 5e+03))))
        (:then_1
          (Audio|PlaySoundatLocation "/Game/VRDemo_Assets/Audio/baseballimpact_soft_Cue.baseballimpact_soft_Cue" (stale Collision|EventHit HitLocation) "0, 0, 0" (Math|Float|Clamp(Float) (/ (Math|Vector|VectorLength (stale Collision|EventHit NormalImpulse)) 2e+03)) 0.97))))))

(fn ConstructionScript)